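; BP_MovableDoor is a door moved by a Transporter, which applies the GE_Dusty gameplay effect to itself when it is in motion between endpoints.
; Tick compares the actor's location with the Transporter's StartPoint and EndPoint using zero tolerance.
; An EffectIsActive flag limits this to one application per trip and resets at either endpoint, without explicitly removing the effect.
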(event EventTick
  (params (DeltaSeconds :type Float%20%28single-precision%29))
  (bind _returnvalue (Transformation|GetActorLocation))
  (bind _returnvalue_2 (Transformation|GetActorLocation))
  (bind _transporter (Variables|Default|GetTransporter))
  (bind _endpoint (Variables|/Script/SuperAdventure.TransporterComponent|GetEndPoint _transporter))
  (bind _startpoint (Variables|/Script/SuperAdventure.TransporterComponent|GetStartPoint _transporter))
  (bind _returnvalue_3 (Utilities|Operators|EqualEqual _returnvalue _startpoint 0.0))
  (bind _returnvalue_4 (Utilities|Operators|EqualEqual _returnvalue_2 _endpoint 0.0))
  (bind _returnvalue_5 (not _returnvalue_4))
  (bind _returnvalue_6 (not _returnvalue_3))
  (bind _returnvalue_7 (and _returnvalue_5 _returnvalue_6))
  (if (and (not (Variables|Default|GetEffectIsActive)) _returnvalue_7)
    (GameplayEffects|ApplyGameplayEffectToSelf :self (Variables|Default|GetAbilitySystem) :GameplayEffectClass "/Game/GameplayElements/GE_Dusty.GE_Dusty_C")
    (Variables|Default|SetEffectIsActive true)
    (elif (not _returnvalue_7)
      (Variables|Default|SetEffectIsActive false))))

(fn ConstructionScript)